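; BP_Ball is the physics-driven game ball that destroys BP_Target actors and notifies player state and game state.
; StartMoving launches it by impulse and captures its speed, which Tick enforces by renormalizing velocity and hits raise.
; PaddleBoost speeds it up and briefly pauses Tick to redirect it toward a target from FindClosestTarget, which returns at the first qualifying one.
; Overlapping BP_ResetBallTrigger restores the initial transform and reports out of bounds.
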(event `self.ReceiveBeginPlay`
  ;[1 1 1] Set some initial properties
  (set `self.InitialTransform` (`SceneComponent.K2_GetComponentToWorld` (`self.Ball`)))
  (bind _asbb_player_state (cast `/Game/Blueprints/BB_PlayerState` (`|GetArrayItem` (`GameStateBase.PlayerArray` (`GameplayStatics.GetGameState`)))))
  (set `self.PlayerState` _asbb_player_state))

(event `Increase Speed`
  ;[1 1 1] Increase ball speed on collision with objects
  (set `self.DesiredSpeed` (+ (`self.DesiredSpeed`) (`self.IncreaseSpeedRate`))))

(event `PaddleBoost`
  (`self.SetActorTickEnabled` false) ; Issue where tick would calculate before this would complete and cause speed issues
  (`self.Increase Speed`)
  (bind _outactors (`GameplayStatics.GetAllActorsOfClass` "/Game/Blueprints/BP_Target.BP_Target_C"))
  (`self.FindClosestTarget` _outactors)
  (`PrimitiveComponent.SetPhysicsLinearVelocity` (`self.Ball`) (* (`KismetMathLibrary.Normal` (- (`self.ClosestTargetPosition`) (`self.K2_GetActorLocation`))) (`self.DesiredSpeed`)) false "None")
  (`KismetSystemLibrary.Delay` 0.1)
  (`self.SetActorTickEnabled` true)
  (set `self.ClosestTargetDistance` 100000000.0) ; Reset for later invocations
)

(event `self.ReceiveTick`
  (params (DeltaSeconds :type "Float (single-precision)"))
  (bind _ball (`self.Ball`))
  ;[1 1 1] Keeps ball speed at constant rate
  (if (`self.IsMoving`)
    (bind _returnvalue (`PrimitiveComponent.GetPhysicsLinearVelocity` _ball "None"))
    (`PrimitiveComponent.SetPhysicsLinearVelocity` _ball (* (`KismetMathLibrary.Normal` _returnvalue) (`self.DesiredSpeed`)) false "None")))

(event `StartMoving`
  (bind _ball (`self.Ball`))
  ;[1 1 1] Gets the ball rolling
  (`PrimitiveComponent.AddImpulse` _ball (* (`self.StartDirection`) (`self.StartForce`)) "None" false)
  (`KismetSystemLibrary.Delay` 0.2) ; Need to wait for the ball to actually start moving before setting the speed
  (bind _returnvalue (`PrimitiveComponent.GetPhysicsLinearVelocity` _ball "None"))
  (set `self.DesiredSpeed` (`KismetMathLibrary.VSize` _returnvalue))
  (set `self.IsMoving` true))

(event `self.Ball.OnComponentHit`
  (params (HitComponent :type "PrimitiveComponent Object Reference") (OtherActor :type "Actor Object Reference") (OtherComp :type "PrimitiveComponent Object Reference") (NormalImpulse :type "Vector Structure") (Hit :type "HitResult Structure (by ref)"))
  ;[1 1 1] When hitting targets
  (bind _asbp_target (cast `/Game/Blueprints/BP_Target` OtherActor)
    (:`then`
      (if (not (== (`self.MostRecentTarget`) _asbp_target))
        (bind _output_get (set `self.MostRecentTarget` _asbp_target))
        (`/Game/Blueprints/BP_Target.Destroy` _output_get)
        (message `/Game/Blueprints/BI_TargetHit.Target Hit` (`self.PlayerState`))
        (message `/Game/Blueprints/BI_TargetHit.Target Hit` (`GameplayStatics.GetGameState`))
        (`self.Increase Speed` :!label _label) ; Regardless of what you hit, increase speed
      ))
    (:`CastFailed`
      (goto _label))))

(event `self.Ball.OnComponentBeginOverlap`
  (params (OverlappedComponent :type "PrimitiveComponent Object Reference") (OtherActor :type "Actor Object Reference") (OtherComp :type "PrimitiveComponent Object Reference") (OtherBodyIndex :type Integer) (bFromSweep :type Boolean) (SweepResult :type "HitResult Structure (by ref)"))
  ;[1 1 1] Did we go out of bounds?
  (cast `/Game/Blueprints/BP_ResetBallTrigger` OtherActor)
  (`self.Reset`)
  (message `/Game/Blueprints/BI_OutOfBounds.OutOfBounds` (`self.PlayerState`)))

(event `Reset`
  (bind _ball (`self.Ball`))
  ;[1 1 1] Reset ball position
  (`PrimitiveComponent.SetPhysicsLinearVelocity` _ball (0.0 0.0 0.0) false "None")
  (`PrimitiveComponent.SetPhysicsAngularVelocityInRadians` _ball (0.0 0.0 0.0) false "None")
  (`self.K2_SetActorTransform` (`self.InitialTransform`) false true)
  (`KismetSystemLibrary.Delay` (`self.ResetDelay`))
  (set `self.IsMoving` false))

(fn `UserConstructionScript`)