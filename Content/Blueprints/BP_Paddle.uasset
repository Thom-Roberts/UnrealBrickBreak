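; BP_Paddle is a player-controlled paddle that spawns and launches a ball.
; On BeginPlay it spawns a scaled-down Ball at the BallSpawn location and keeps a reference to it, without attaching it.
; The Right axis slides the Cube component along relative Y by MoveSpeed, without sweep or delta-time scaling.
; The SpawnBall action starts that existing ball moving if it is not already, rather than spawning another.
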(event `self.ReceiveBeginPlay`
  (bind _returnvalue_location (`KismetMathLibrary.BreakTransform` (`SceneComponent.K2_GetComponentToWorld` (`self.BallSpawn`))))
  ;[1 1 1] Spawn ball on game start
  (bind _returnvalue (`|SpawnActorFromClass` (`self.Ball`) (`KismetMathLibrary.MakeTransform` _returnvalue_location (struct) (0.25 0.25 0.25)) "Undefined" "OverrideRootScale" null null))
  (set `self.SpawnedBall` _returnvalue))

(event `InputAxis|Right`
  (params (AxisValue :type "Float (single-precision)"))
  ;[1 1 1] Moving left/right
  (`SceneComponent.K2_AddRelativeLocation` (`self.Cube`) (`KismetMathLibrary.MakeVector` 0.0 (* AxisValue (`self.MoveSpeed`))) false false))

(event `InputAction|SpawnBall`
  (params (Key :type "Key Structure"))
  (bind _spawnedball (`self.SpawnedBall`))
  ;[1 1 1] Start the ball moving when the player presses the key
  (:`Pressed`
    (if (not (`/Game/Blueprints/BP_Ball.IsMoving` _spawnedball))
      (`/Game/Blueprints/BP_Ball.StartMoving` _spawnedball))))

(fn `UserConstructionScript`)