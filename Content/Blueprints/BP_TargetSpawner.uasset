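; Brick spawner for a block-breaking game that fills a grid of scaled Target actors on BeginPlay.
; SpawnBricks runs nested column and row loops, placing each actor at the location from GetSpawnOffset, then writes the total brick count to NumBlocks on BB_GameState.
; GetSpawnOffset holds math offsetting SpawnPoint's relative location along Y by column and Z by row, though that node appears unconnected.
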(event `self.ReceiveBeginPlay`
  (`self.SpawnBricks`))

(event `SpawnBricks`
  (bind _numberofrows (`self.NumberOfRows`))
  (bind _numberofcolumns (`self.NumberOfColumns`))
  ;[1 1 1] Setup brick spawn
  (for _index (range _numberofcolumns)
    (for _index_2 (range _numberofrows)
      (`|SpawnActorFromClass` (`self.Target`) (`KismetMathLibrary.MakeTransform` (`self.GetSpawnOffset` _index _index_2) (struct) (0.25 0.5 0.1)) "Undefined" "OverrideRootScale" null null)))
  ;[1 1 1] Notify game state of how many blocks we have
  (bind _asbb_game_state (cast `/Game/Blueprints/BB_GameState` (`GameplayStatics.GetGameState`)))
  (set `/Game/Blueprints/BB_GameState.NumBlocks` (* _numberofcolumns _numberofrows) _asbb_game_state))

(fn `UserConstructionScript`)